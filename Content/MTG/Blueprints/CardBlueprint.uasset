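; Card actor for a Magic: The Gathering style game that players hover, grab and release.
; It inits from CardId, then applies the fetched texture to the front plane through a dynamic material and links the HUD_Card info widget.
; Hover shows the widget and cone unless the owning character is grabbing, and nudges hand cards.
; Grab attaches the card to the player's Scene with a zone-dependent offset; Release detaches it at a fixed height.
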(event OnBeginCursorOver(Box)
  (params (TouchedComponent :type Primitive%20Component%20Object%20Reference))
  ;[1 1 1] Hover Card
  (bind _asmtgplayer_character_bp (Utilities|Casting|CastToMTGPlayerCharacter_BP (Components|GetOwner)))
  (bind _isholding (Default|IsGrabbingObject _asmtgplayer_character_bp))
  (if (not _isholding)
    (Rendering|SetVisibility (Variables|Default|GetCardInfoWidget) true false)
    (Rendering|SetVisibility (Variables|Default|GetCone) true false)
    (Utilities|Casting|CastToMTGHandActorComponent (Variables|Default|GetCurrentZone))
    (Transformation|AddLocalOffset (Variables|Default|GetRootTransform) "0.000000,-55.000000, 0" false false)))

(event OnEndCursorOver(Box)
  (params (TouchedComponent :type Primitive%20Component%20Object%20Reference))
  ;[1 1 1] Hover Card
  (bind _asmtgplayer_character_bp (Utilities|Casting|CastToMTGPlayerCharacter_BP (Components|GetOwner)))
  (bind _isholding (Default|IsGrabbingObject _asmtgplayer_character_bp))
  (if (not _isholding)
    (Rendering|SetVisibility (Variables|Default|GetCardInfoWidget) false false)
    (Rendering|SetVisibility (Variables|Default|GetCone) false false)
    (Utilities|Casting|CastToMTGHandActorComponent (Variables|Default|GetCurrentZone))
    (Transformation|AddLocalOffset (Variables|Default|GetRootTransform) "0.000000,55.000000, 0" false false)))

(event Custom|OnCardTextureFetched_Event_0
  (params (CardSide :type ECardSide%20Enum :default "Front") (Texture :type Texture%202D%20Object%20Reference))
  (CallFunction|SetFrontsideTexture CardSide Texture)
  (Rendering|SetVisibility (Variables|Default|GetCardInfoWidget) false false)
  (Rendering|SetVisibility (Variables|Default|GetCone) false false)
  (bind _ashud_card (Utilities|Casting|CastToHUD_Card (UserInterface|GetUserWidgetObject (Variables|Default|GetCardInfoWidget))))
  (Default|SetCard _ashud_card self))

(event EventBeginPlay
  (Class|Card|InitCard (Variables|Default|GetCardId))
  (EventDispatchers|AssignOnCardTextureFetched (delegate Custom|OnCardTextureFetched_Event_0)))

(event Collision|EventActorBeginOverlap
  (params (OtherActor :type Actor%20Object%20Reference)))

(event EventTick
  (params (DeltaSeconds :type Float%20%28single-precision%29)))

(fn ConstructionScript)

(fn SetFrontsideTexture
  (params (CardSide :type ECardSide%20Enum :default "Front") (Texture :type Texture%20Object%20Reference))
  (bind _plane (Variables|Default|GetPlane))
  (Utilities|IsValid Texture
    (:Is%20Valid
      (switch Utilities|FlowControl|Switch|SwitchonECardSide CardSide
        (:Front
          (bind _returnvalue (Rendering|Material|CreateDynamicMaterialInstance _plane 0 (Rendering|Material|GetMaterial _plane 0) "None" :!class /Script/Engine.PrimitiveComponent))
          (Rendering|Material|SetVectorParameterValue :self _returnvalue :ParameterName "Color" :!class /Script/Engine.MaterialInstanceDynamic)
          (Rendering|Material|SetTextureParameterValue _returnvalue "Texture" Texture)
          (Rendering|Material|SetScalarParameterValue _returnvalue "Roughness" 1.0 :!class /Script/Engine.MaterialInstanceDynamic)
          (Rendering|Material|SetMaterial (Variables|Default|GetPlane) 0 _returnvalue))))))

(fn Release
  (bind _returnvalue (Transformation|GetActorLocation))
  (bind (_x _y) (Math|Vector|BreakVector _returnvalue))
  (Transformation|DetachFromActor "KeepWorld" "KeepRelative" "KeepRelative")
  (Transformation|SetActorLocation (Math|Vector|MakeVector _x _y 1e+01) false false)
  (Transformation|SetRelativeLocation (Variables|Default|GetRootTransform) "0, 0, 0" false false))

(fn Grab
  (params (PC :type MTG%20Player%20Character%20BP%20Object%20Reference))
  (bind _roottransform (Variables|Default|GetRootTransform))
  (Transformation|AttachComponentToComponent (Variables|/Game/MTG/Blueprints/MTGPlayerCharacter_BP.MTGPlayerCharacter_BP_C|GetScene PC) "None" "KeepWorld" "KeepRelative" "KeepRelative" false)
  (Utilities|Casting|CastToMTGHandActorComponent (Variables|Default|GetCurrentZone)
    (:then
      (Transformation|SetRelativeLocation _roottransform "0, 0,-5.000000" false false))
    (:CastFailed
      (Transformation|SetRelativeLocation _roottransform "0, 0,5.000000" false false))))