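; Playground actor for the MTG card game that represents the player's play area and turns cards entering its battlefield box into casts.
; BeginPlay stores the first player's character as owner, and Setup initializes that player's Library from a deck.
; A card from a hand zone overlapping BattlefieldBox is cast to the owner's Battlefield, then snapped to BattlefieldScene and offset along Y by card count to form a row.
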(event OnComponentBeginOverlap(BattlefieldBox)
  (params (OverlappedComponent :type Primitive%20Component%20Object%20Reference) (OtherActor :type Actor%20Object%20Reference) (OtherComp :type Primitive%20Component%20Object%20Reference) (OtherBodyIndex :type Integer) (bFromSweep :type Boolean) (SweepResult :type Hit%20Result%20Structure%20%28by%20ref%29))
  (bind _owningplayer (Variables|Default|GetOwningPlayer))
  (bind _battlefieldbox (Variables|Default|GetBattlefieldBox))
  (bind _battlefield (Variables|/Script/UnrealMTG.MTGPlayerCharacter|GetBattlefield _owningplayer))
  (bind _boxextent (Variables|/Script/Engine.BoxComponent|GetBoxExtent _battlefieldbox))
  (bind (_x _y) (Math|Vector|BreakVector _boxextent))
  ;[1 1 1] Cast To Battlefield
  (bind _ascard (Utilities|Casting|CastToCard OtherActor))
  (bind _asmtghand_actor_component (Utilities|Casting|CastToMTGHandActorComponent (Variables|/Script/UnrealMTG.Card|GetCurrentZone _ascard)))
  (Class|MTGHandActorComponent|CastCards _asmtghand_actor_component _battlefield (Utilities|Set|MakeSet _ascard))
  (bind _result (Utilities|Set|ToArray (Utilities|Set|MakeSet _ascard)))
  (for _array_element _result
    (Transformation|AttachComponentToComponent _array_element (Variables|Default|GetBattlefieldScene) "None" "SnapToTarget" "KeepRelative" "KeepRelative" true)
    (Transformation|AddActorLocalOffset _array_element (Math|Vector|MakeVector (/ _x 2.0) (+ (* (Utilities|Set|Length (Variables|/Script/UnrealMTG.AbstractPlaygroundActorComponent|GetCards _battlefield)) 105.0) (* _y -1.0)) 0.0) false false)))

(event EventBeginPlay
  (bind _asmtgplayer_character_bp (Utilities|Casting|CastToMTGPlayerCharacter_BP (Game|GetPlayerCharacter (Variables|Default|GetPlayer%20Index))))
  (Variables|Default|SetOwningPlayer _asmtgplayer_character_bp))

(event Collision|EventActorBeginOverlap
  (params (OtherActor :type Actor%20Object%20Reference)))

(event EventTick
  (params (DeltaSeconds :type Float%20%28single-precision%29)))

(fn ConstructionScript)

(fn Setup
  (params (Deck :type Set%20of%20Card%20Object%20References))
  (Class|MTGLibraryActorComponent|Init (Variables|/Script/UnrealMTG.MTGPlayerCharacter|GetLibrary (Variables|Default|GetOwningPlayer)) Deck))